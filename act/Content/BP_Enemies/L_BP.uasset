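; L_BP is a shared helper library in the enemies folder, offering a player cast and area-of-effect spawning.
; CastToPlayer returns player pawn zero as BP_ThirdPersonCharacter with a success flag.
; SpawnAOEOverlap switches on shape and forwards placement, line-of-sight, instigator, hit delegate and debug settings to MYGameState spawners.
; The Capsule and Box cases are crossed: Capsule calls SpawnBoxAOE and Box calls SpawnCapsuleAOE.
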(fn `Cast to Player`
  (returns (`Cast Return` :type Boolean) (`AsBP Third Person Character` :type "/Game/ThirdPerson/Blueprints/BP_ThirdPersonCharacter Object Reference"))
  (bind _asbp_third_person_character (cast `/Game/ThirdPerson/Blueprints/BP_ThirdPersonCharacter` (`GameplayStatics.GetPlayerPawn` null))
    (:`then`
      (return true _asbp_third_person_character))
    (:`CastFailed`
      (return false _asbp_third_person_character))))

(fn `Spawn AOE Overlap`
  (params (AOE :type "/Game/BP_Enemies/E_AOEState Enum" :default "NewEnumerator0") (Location :type "Vector Structure") (Radius :type "Float (double-precision)") (`Require LOS` :type Boolean) (Instigator :type "Actor Object Reference") (`Hit Delegate` :type "Delegate (by ref)") (`Draw Debug Time` :type "Float (double-precision)") (Extent :type "Vector Structure") (`Half Height` :type "Float (double-precision)"))
  (locals (`Game State` :type "/Game/BP_Enemies/MYGameState Object Reference"))
  (set `local.Game State` (cast `/Game/BP_Enemies/MYGameState` (`GameplayStatics.GetGameState` null) :!pure true))
  (switch `/Game/BP_Enemies/E_AOEState` (`local.AOE`)
    (:`NewEnumerator0`
      (`/Game/BP_Enemies/MYGameState.Spawn AOE` (`local.Game State`) (`local.Location`) (`local.Radius`) (`local.Require LOS`) (`local.Instigator`) (`local.Hit Delegate`) (`local.Draw Debug Time`)))
    (:`NewEnumerator1`
      (`/Game/BP_Enemies/MYGameState.Spawn Box AOE` (`local.Game State`) (`local.Location`) (`local.Require LOS`) (`local.Instigator`) (`local.Hit Delegate`) (`local.Draw Debug Time`) (`local.Extent`)))
    (:`NewEnumerator2`
      (`/Game/BP_Enemies/MYGameState.Spawn Capsule AOE` (`local.Game State`) (`local.Location`) (`local.Radius`) (`local.Half Height`) (`local.Draw Debug Time`) (`local.Instigator`) (`local.Hit Delegate`) (`local.Require LOS`)))))