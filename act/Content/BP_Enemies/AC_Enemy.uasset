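; Enemy actor component that tracks health and the owner's horizontal position relative to the player character.
; Every tick it computes the 2D distance to the player, the angle off the owner's forward vector via dot product and arccosine, and a left/right side from the dot with the right vector.
; Health starts at maximum, and GetDamage subtracts damage with clamping, returning true when health is depleted.
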(event `self.ReceiveBeginPlay`
  (set `self.Health` (`self.Max Health`)))

(event `self.ReceiveTick`
  (params (DeltaSeconds :type "Float (single-precision)"))
  (`self.Get Distance and Angles to Player`))

(fn `Get Damage`
  (params (Damage :type "Float (double-precision)"))
  (returns (`Dead?` :type Boolean))
  (bind _output_get (set `self.Health` (`KismetMathLibrary.FClamp` (- (`self.Health`) Damage) 0.0 (`self.Max Health`))))
  (if (> _output_get 0.0)
    (return false)
    (else
      (return true))))

(fn `Get Distance and Angles to Player`
  (bind (_cast_return _asbp_third_person_character) (`/Game/ThirdPerson/Blueprints/L_BP.Cast to Player`))
  (bind _returnvalue (`self.GetOwner`))
  (bind (_returnvalue_x _returnvalue_y) (`KismetMathLibrary.BreakVector` (`Actor.GetActorForwardVector` _returnvalue)))
  (bind (_returnvalue_x_2 _returnvalue_y_2) (`KismetMathLibrary.BreakVector` (`Actor.GetActorRightVector` _returnvalue)))
  (bind (_returnvalue_x_3 _returnvalue_y_3) (`KismetMathLibrary.BreakVector` (`Actor.K2_GetActorLocation` _returnvalue)))
  (bind (_returnvalue_x_4 _returnvalue_y_4) (`KismetMathLibrary.BreakVector` (`Actor.K2_GetActorLocation` _asbp_third_person_character)))
  (bind _returnvalue_2 (- _returnvalue_y_4 _returnvalue_y_3))
  (bind _returnvalue_3 (- _returnvalue_x_4 _returnvalue_x_3))
  (bind _returnvalue_4 (`KismetMathLibrary.MakeVector2D` _returnvalue_3 _returnvalue_2))
  (if _cast_return
    (set `self.Distance` (`KismetMathLibrary.Sqrt` (+ (`KismetMathLibrary.Square` _returnvalue_3) (`KismetMathLibrary.Square` _returnvalue_2))))
    (set `self.Angle` (`KismetMathLibrary.DegAcos` (`self.Get Two Points' Cos` _returnvalue_4 (`KismetMathLibrary.MakeVector2D` _returnvalue_x _returnvalue_y))))
    (if (>= (`self.Get Two Points' Cos` _returnvalue_4 (`KismetMathLibrary.MakeVector2D` _returnvalue_x_2 _returnvalue_y_2)) 0.0)
      (set `self.Right or Left` "NewEnumerator0")
      (else
        (set `self.Right or Left` "NewEnumerator1")))))

(fn `Get Two Points' Cos`
  (params (A :type "Vector2D Structure") (B :type "Vector2D Structure"))
  (returns (ReturnValue :type "Float (double-precision)"))
  (return (/ (`KismetMathLibrary.DotProduct2D` A B) (* (`KismetMathLibrary.VSize2D` A) (`KismetMathLibrary.VSize2D` B)))))