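; Forest Giant golem enemy Blueprint that feeds player sightings to its AI Blackboard and selects damage per attack type.
; PawnSensing sets the "Look?" key when it sees a Player-tagged pawn; seeing any other pawn clears it after a retriggerable three-second delay.
; Attack looks up DT_Attack rows for Floor, Stone and Sweep, setting Damage for the first two; the Sweep row's result is unused.
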(event `self.PawnSensing.OnSeePawn`
  (params (Pawn :type "Pawn Object Reference"))
  (if (`self.ActorHasTag` Pawn "Player")
    (`self.Set Blackboard Bool` "Look?" true)
    (else
      (`KismetSystemLibrary.RetriggerableDelay` 3.0)
      (`self.Set Blackboard Bool` "Look?"))))

(fn `Attack`
  (params (`Cur Attack` :type "/Game/BP_Enemies/ForestGolems/E_Attacks_For Enum" :default "NewEnumerator0"))
  (locals (Damage :type "Float (double-precision)"))
  (switch `/Game/BP_Enemies/ForestGolems/E_Attacks_For` `Cur Attack`
    (:`NewEnumerator0`
      (bind _returnvalue (`|GetDataTableRow` "/Game/BP_Enemies/DT_Attack.DT_Attack" "For_Floor")
        (:`then`
          (set `local.Damage` (`.Damage_7_DDF83C93496F4117C59CC599B9D5BA56` (break `/Game/BP_Enemies/F_Attacks` _returnvalue))))))
    (:`NewEnumerator1`
      (bind _returnvalue_2 (`|GetDataTableRow` "/Game/BP_Enemies/DT_Attack.DT_Attack" "For_Stone")
        (:`then`
          (set `local.Damage` (`.Damage_7_DDF83C93496F4117C59CC599B9D5BA56` (break `/Game/BP_Enemies/F_Attacks` _returnvalue_2))))))
    (:`NewEnumerator3`
      (bind _returnvalue_3 (`|GetDataTableRow` "/Game/BP_Enemies/DT_Attack.DT_Attack" "For_Sweep")))))

(fn `Set Blackboard Bool`
  (params (KeyName :type "Name (by ref)") (BoolValue :type Boolean))
  (`BlackboardComponent.SetValueAsBool` (`self.Blackboard`) KeyName BoolValue))

(fn `UserConstructionScript`)