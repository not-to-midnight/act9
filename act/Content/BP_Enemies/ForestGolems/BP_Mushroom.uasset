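; BP_Mushroom is a forest golem mushroom hazard that rises into place and pulses poison damage around itself.
; On BeginPlay it reads damage from the DT_Attack table and, if found, plays a timeline that lifts it through a Lerp helper.
; A looping timer spawns a small line-of-sight AOE overlap each second, applying that damage to hit actors tagged "None".
; GetLocationAndDestiny stores the start location and rise height, but is not called here.
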(event `self.ReceiveBeginPlay`
  (bind (_location_x _location_y _location_z) (`KismetMathLibrary.BreakVector` (`self.Location`)))
  (`KismetSystemLibrary.K2_SetTimerDelegate` (delegate `Creat Poison Fog`) 1.0 true)
  (bind _returnvalue (`|GetDataTableRow` "/Game/BP_Enemies/DT_Attack.DT_Attack" "For_Mushroom")
    (:`then`
      (set `self.Damage` (`.Damage_7_DDF83C93496F4117C59CC599B9D5BA56` (break `/Game/BP_Enemies/F_Attacks` _returnvalue)))
      (bind (_direction `_新建轨道_0`) (`Timeline|Rise` :!via `PlayFromStart`)
        (:`Update`
          (`self.K2_SetActorLocation` (`KismetMathLibrary.VLerp` (`self.Location`) (`KismetMathLibrary.MakeVector` _location_x _location_y (+ _location_z (`self.Height`))) `_新建轨道_0`)))))))

(event `Creat Poison Fog`
  (`/Game/BP_Enemies/L_BP.Spawn AOE Overlap` "NewEnumerator0" (`self.K2_GetActorLocation`) 50.0 true self (delegate `Wanna Make Damage`) (`self.Draw Debug Time`)))

(event `Wanna Make Damage`
  (params (`Hit Actor` :type "Actor Object Reference"))
  (bind _returnvalue (`self.GetInstigatorController`))
  (if (`self.ActorHasTag` `Hit Actor` "None")
    (`GameplayStatics.ApplyDamage` `Hit Actor` (`self.Damage`) _returnvalue _returnvalue)))

(fn `Get Location and Destiny`
  (params (Height :type "Float (double-precision)"))
  (set `self.Height` Height)
  (set `self.Location` (`self.K2_GetActorLocation`))
  (return))

(fn `UserConstructionScript`)